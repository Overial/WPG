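; BP_Pickup is a world item that adds itself to a pawn's inventory on overlap.
; On BeginPlay it looks up its ItemTag in the game instance's item map to set the name exposed by GetObjectName.
; When a pawn with a BP_InventoryComponent enters PickupBox, it adds the tagged item and count, plays a hit particle and pickup sound, then destroys itself.
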(event OnComponentBeginOverlap(PickupBox)
  (params (OverlappedComponent :type Primitive%20Component%20Object%20Reference) (OtherActor :type Actor%20Object%20Reference) (OtherComp :type Primitive%20Component%20Object%20Reference) (OtherBodyIndex :type Integer) (bFromSweep :type Boolean) (SweepResult :type Hit%20Result%20Structure%20%28by%20ref%29))
  (bind _returnvalue (Actor|GetComponentbyClass OtherActor "/Game/WPG/Blueprints/Inventory/BP_InventoryComponent.BP_InventoryComponent_C"))
  (if (Utilities|ClassIsChildOf (Utilities|GetClass OtherActor) "/Script/Engine.Pawn")
    (Utilities|IsValid _returnvalue
      (:Is%20Valid
        (Default|AddItem _returnvalue (Variables|Pickup|GetItemTag) (Variables|Pickup|GetItemCount))
        (Effects|SpawnEmitteratLocation "/Game/FXVarietyPack/Particles/P_ky_hit2.P_ky_hit2" (Transformation|GetActorLocation) (Math|Random|RandomRotator false) "0.500000,0.500000,0.500000")
        (Audio|PlaySound2D "/Engine/VREditor/Sounds/UI/Object_PickUp.Object_PickUp" 1.0 1.0 0.0 0 0)
        (Actor|DestroyActor)))))

(event EventBeginPlay
  (bind _asbp_wpggame_instance (Utilities|Casting|CastToBP_WPGGameInstance (Game|GetGameInstance)))
  (if (.ReturnValue (Utilities|Map|Find (Default|GetItems _asbp_wpggame_instance) (Variables|Pickup|GetItemTag)))
    (Variables|Default|SetObjectName (.Value (Utilities|Map|Find (Default|GetItems _asbp_wpggame_instance) (Variables|Pickup|GetItemTag))))))

(fn ConstructionScript)

(fn GetObjectName
  (return (Variables|Default|GetObjectName)))