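; BP_Spawner is a spawner that periodically creates ObjectToSpawn actors inside its box until MaxObjectCount is reached.
; A looping timer spawns each at a random XY within half the box extent, at the box's center height, then stops at the cap.
; Destroy events decrement the count and restart the timer below the cap.
; On BeginPlay, matching actors already overlapping the box get destroy bindings without being added to the count.
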(event EventBeginPlay
  (CallFunction|ProcessObjectsfromLevel)
  (CallFunction|InitSpawnTimer))

(fn ConstructionScript)

(fn InitSpawnTimer
  (bind _returnvalue (Utilities|Time|SetTimerbyFunctionName 0 "SpawnObject" (Variables|Settings|GetSpawnDelay) true))
  (Variables|Default|SetSpawnObjectTimer _returnvalue))

(fn SpawnObject
  (bind _box (Variables|Default|GetBox))
  (bind _returnvalue (Transformation|GetWorldLocation _box))
  (bind _boxextent (Variables|/Script/Engine.BoxComponent|GetBoxExtent _box))
  (bind _returnvalue_2 (/ _boxextent "2.000000,2.000000,2.000000"))
  (bind _returnvalue_3 (Math|Random|RandomPointinBoundingBox _returnvalue _returnvalue_2))
  (bind (_x _y) (Math|Vector|BreakVector _returnvalue_3))
  (bind _returnvalue_4 (Game|SpawnActorfromClass (Variables|Settings|GetObjectToSpawn) (Math|Transform|MakeTransform (Math|Vector|MakeVector _x _y (.Z (Math|Vector|BreakVector _returnvalue))) (Math|Rotator|MakeRotator 0.0 0.0 (Math|Random|RandomFloat)) "1.000000,1.000000,1.000000") "AdjustIfPossibleButDontSpawnIfColliding" "MultiplyWithRoot" 0 0))
  (Game|BindEventtoOnDestroyed _returnvalue_4 (EventDispatchers|CreateEvent :!event OnObjectDestroyed))
  (Utilities|FlowControl|Sequence
    (:then_0
      (bind _output_get (Variables|Settings|SetObjectCount (+ (Variables|Settings|GetObjectCount) 1)))
      (if (>= _output_get (Variables|Settings|GetMaxObjectCount))
        (Utilities|Time|ClearandInvalidateTimerbyHandle (Variables|Default|GetSpawnObjectTimer))
        (Development|PrintString "Spawn timer stopped" false)
        (elif (not (Utilities|Time|IsValidTimerHandle (Variables|Default|GetSpawnObjectTimer)))
          (CallFunction|InitSpawnTimer)
          (Development|PrintString "Spawn timer restarted"))))
    (:then_1
      (Development|PrintString (Utilities|String|Append "Object \"" (Utilities|GetDisplayName _returnvalue_4) "\" was spawned (" (Utilities|String|ToString(Integer) (Variables|Settings|GetObjectCount)) " of " (Utilities|String|ToString(Integer) (Variables|Settings|GetMaxObjectCount)) ")") false))))

(fn OnObjectDestroyed
  (params (DestroyedActor :type Actor%20Object%20Reference))
  (bind _output_get (Variables|Settings|SetObjectCount (- (Variables|Settings|GetObjectCount) 1)))
  (if (< _output_get (Variables|Settings|GetMaxObjectCount))
    (CallFunction|InitSpawnTimer)))

(fn ProcessObjectsfromLevel
  (for _array_element (Collision|GetOverlappingActors (Variables|Default|GetBox) 0 :!class /Script/Engine.PrimitiveComponent)
    (if (Utilities|ClassIsChildOf (Utilities|GetClass _array_element) (Variables|Settings|GetObjectToSpawn))
      (Game|BindEventtoOnDestroyed _array_element (EventDispatchers|CreateEvent :!event OnObjectDestroyed)))))