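; Inventory component that stores items in a map from gameplay tag to count, with events to add and remove them.
; AddItem writes the passed count as the item's value, replacing any existing count rather than summing.
; RemoveItem deletes the entry when nothing would remain, but otherwise stores the passed count instead of the remainder.
; Each outcome, including a missing item, is logged without on-screen printing.
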(event Custom|AddItem
  (params (Item :type Gameplay%20Tag%20Structure) (Count :type Integer))
  (Utilities|Map|Add (Variables|Default|GetInventory) Item Count)
  (Development|PrintString (Utilities|String|Append "Item \"" (Utilities|String|ToString(Name) (GameplayTags|GetTagName Item)) "\" (" (Utilities|String|ToString(Integer) Count) "} was added to the inventory") false))

(event Custom|RemoveItem
  (params (Item :type Gameplay%20Tag%20Structure) (Count :type Integer))
  (bind _inventory (Variables|Default|GetInventory))
  (bind (_value _returnvalue) (Utilities|Map|Find _inventory Item))
  (if _returnvalue
    (if (> (- _value Count) 0) ; Если какое-то количество осталось\nпосле вычитания, обновляем Map
      (Utilities|Map|Add (Variables|Default|GetInventory) Item Count)
      (Development|PrintString (Utilities|String|Append "Item \"" (Utilities|String|ToString(Name) (GameplayTags|GetTagName Item)) "\" (" (Utilities|String|ToString(Integer) Count) "} was removed from the inventory") false)
      (else
        (Utilities|Map|Remove (Variables|Default|GetInventory) Item)
        (Development|PrintString (Utilities|String|Append "Item \"" (Utilities|String|ToString(Name) (GameplayTags|GetTagName Item)) "\" (" (Utilities|String|ToString(Integer) Count) ") is not longer present in the inventory") false)))
    (else
      (Development|PrintString (Utilities|String|Append "Item \"" (Utilities|String|ToString(Name) (GameplayTags|GetTagName Item)) "\" (" (Utilities|String|ToString(Integer) Count) ") not found in the inventory") false))))