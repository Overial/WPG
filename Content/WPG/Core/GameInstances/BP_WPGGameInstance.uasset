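; BP_WPGGameInstance is the game instance that loads item and command data from data tables when the game starts.
; On Init it walks every row of the items table, mapping each tag to its readable name, and collects every commands table row into a Commands collection.
; GetItems and GetCommands expose these cached collections.
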(event EventInit
  (CallFunction|ProcessItemData)
  (CallFunction|ProcessCommandData))

(fn ProcessItemData
  (bind _itemsdatatable (Variables|Default|GetItemsDataTable))
  (bind _outrownames (DataTable|GetDataTableRowNames _itemsdatatable))
  (for _array_element _outrownames
    (bind _returnvalue (Utilities|GetDataTableRow _itemsdatatable _array_element)
      (:then
        (Utilities|Map|Add (Variables|Default|GetItems) (.Tag (Utilities|Struct|BreakFItem _returnvalue)) (.ReadableName (Utilities|Struct|BreakFItem _returnvalue)))))))

(fn GetItems
  (return (Variables|Default|GetItems)))

(fn ProcessCommandData
  (bind _commandsdatatable (Variables|Default|GetCommandsDataTable))
  (bind _outrownames (DataTable|GetDataTableRowNames _commandsdatatable))
  (for _array_element _outrownames
    (bind _returnvalue (Utilities|GetDataTableRow _commandsdatatable _array_element)
      (:then
        (Utilities|Array|Add (Variables|Default|GetCommands) _returnvalue)))))

(fn GetCommands
  (return (Variables|Default|GetCommands)))